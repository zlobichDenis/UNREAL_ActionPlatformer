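; AIC_Enemy is the enemy AI controller, running the BT_Enemy behavior tree on the BB_Enemy blackboard.
; On possess it caches the BP_ActionChar and mirrors its stun state into the blackboard.
; SetAttackTarget stores the target in both blackboard and controller.
; Each tick, with a valid target, the focal point follows only the target direction's X component, or holds current facing when the character cannot act.
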(event `self.ReceiveBeginPlay`
  (`self.UseBlackboard` "/Game/Blueprints/AI/BB_Enemy.BB_Enemy")
  (`self.RunBehaviorTree` "/Game/Blueprints/AI/BT_Enemy.BT_Enemy"))

(event `self.ReceiveTick`
  (params (DeltaSeconds :type "Float (single-precision)"))
  (`self.SetFocusDirection`))

(event `self.ReceivePossess`
  (params (PossessedPawn :type "Pawn Object Reference"))
  (bind _asbp_action_char (cast `/Game/Blueprints/Characters/BP_ActionChar` PossessedPawn))
  (set `self.ActionChar` _asbp_action_char)
  (add `/Game/Blueprints/Characters/BP_ActionChar.StunStateChanged` _asbp_action_char (delegate `OnStunStateChanged`)))

(event `OnStunStateChanged`
  (params (IsStunned :type Boolean))
  (`BlackboardComponent.SetValueAsBool` (`self.Blackboard`) (`self.IsStunned`) IsStunned))

(fn `SetAttackTarget`
  (params (AttackTarget :type "/Game/Blueprints/Characters/Captain/BP_Captain Object Reference"))
  (`BlackboardComponent.SetValueAsObject` (`self.Blackboard`) (`self.AttackTargetKey`) (`local.AttackTarget`))
  (set `self.AttackTarget` (`local.AttackTarget`)))

(fn `SetFocusDirection`
  (bind _actionchar (`self.ActionChar`))
  (bind _returnvalue_x (`KismetMathLibrary.BreakVector` (`KismetMathLibrary.GetForwardVector` (`KismetMathLibrary.FindLookAtRotation` (`self.K2_GetActorLocation` (`self.ActionChar`)) (`self.K2_GetActorLocation` (`self.AttackTarget`))))))
  (`/Engine/EditorBlueprintResources/StandardMacros.IsValid` (`self.AttackTarget`)
    (:`Is Valid`
      (if (`/Game/Blueprints/Characters/BP_ActionChar.CanAct` (`self.ActionChar`))
        (`self.K2_SetFocalPoint` (+ (`self.K2_GetActorLocation` (`self.ActionChar`)) (`KismetMathLibrary.MakeVector` _returnvalue_x)))
        (else
          (`self.K2_SetFocalPoint` (+ (`self.K2_GetActorLocation` _actionchar) (`self.GetActorForwardVector` _actionchar))))))))

(fn `UserConstructionScript`)